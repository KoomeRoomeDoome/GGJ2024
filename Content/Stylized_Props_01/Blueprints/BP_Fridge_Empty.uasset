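; BP_Fridge_Empty is a configurable fridge prop with bottom, top and freezer doors, a drawer and two spot lights.
; The Construction Script applies exposed variables to yaw each door open, slide the drawer along Y and set the mobility of those parts and the lights.
; It also drives emissive brightness and color material parameters on the body and doors, and shares one set of light settings across both spot lights.
; The event graph has no runtime logic.
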(event EventBeginPlay)

(event Collision|EventActorBeginOverlap
  (params (OtherActor :type Actor%20Object%20Reference)))

(event EventTick
  (params (DeltaSeconds :type Float%20%28single-precision%29)))

(fn ConstructionScript
  (bind _sm_fridge_freezer_door (Variables|Default|GetSM_Fridge_Freezer_Door))
  (bind _sm_fridge_bottom_door (Variables|Default|GetSM_Fridge_Bottom_Door))
  (bind _sm_fridge_top_door (Variables|Default|GetSM_Fridge_Top_Door))
  (bind _spotlight (Variables|Default|GetSpotLight))
  (bind _sm_fridge_drawer (Variables|Default|GetSM_Fridge_Drawer))
  (Utilities|FlowControl|Sequence
    (:then_0
      (Transformation|AddLocalRotation _sm_fridge_bottom_door (Math|Rotator|MakeRotator 0.0 0.0 (* -1.0 (Variables|FRIDGEPARTS|GetBottom%20Door%20Angle))) false false)
      (Transformation|SetMobility _sm_fridge_bottom_door (Variables|FRIDGEPARTS|GetBottom%20Door%20Mobility)))
    (:then_1
      (Transformation|AddLocalRotation _sm_fridge_top_door (Math|Rotator|MakeRotator 0.0 0.0 (* -1.0 (Variables|FRIDGEPARTS|GetTop%20Door%20Angle))) false false)
      (Transformation|SetMobility _sm_fridge_top_door (Variables|FRIDGEPARTS|GetTop%20Door%20Mobility)))
    (:then_2
      (Transformation|AddLocalRotation _sm_fridge_freezer_door (Math|Rotator|MakeRotator 0.0 0.0 (* -1.0 (Variables|FRIDGEPARTS|GetFreezer%20Door%20Angle))) false false)
      (Transformation|SetMobility _sm_fridge_freezer_door (Variables|FRIDGEPARTS|GetFreezer%20Door%20Mobility)))
    (:then_3
      (Rendering|Material|SetScalarParameterValueonMaterials _sm_fridge_freezer_door "Emissive_Brightness" (Variables|FRIDGELIGHT|GetEmissive%20Brightness))
      (Rendering|Material|SetVectorParameterValueonMaterials _sm_fridge_freezer_door "Emissive Color Blend" (Math|Conversions|ToVector(LinearColor) (Math|Conversions|ToLinearColor(Color) (Variables|FRIDGELIGHT|GetEmissive%20Color%20Blend)))))
    (:then_4
      (Rendering|Lighting|SetAttenuationRadius _spotlight (Variables|FRIDGELIGHT|GetLight%20Radius))
      (Rendering|Lighting|SetOuterConeAngle _spotlight (Variables|FRIDGELIGHT|GetLight%20Outer%20Cone))
      (Rendering|Lighting|SetInnerConeAngle _spotlight (Variables|FRIDGELIGHT|GetLight%20Inner%20Cone))
      (Rendering|Components|Light|SetIntensity _spotlight (Variables|FRIDGELIGHT|GetLight%20Intensity))
      (Rendering|Components|Light|SetLightColor _spotlight (Variables|FRIDGELIGHT|GetLight%20Color) true)
      (Transformation|SetMobility _spotlight (Variables|FRIDGELIGHT|GetLight%20Mobility))
      (Class|PointLightComponent|SetSoftSourceRadius _spotlight (Variables|FRIDGELIGHT|GetSoft%20Source%20Radius))
      (Class|PointLightComponent|SetSourceRadius _spotlight (Variables|FRIDGELIGHT|GetSource%20Radius))
      (Class|PointLightComponent|SetSourceLength _spotlight (Variables|FRIDGELIGHT|GetSource%20Length))
      (Class|LightComponent|SetIndirectLightingIntensity _spotlight (Variables|FRIDGELIGHT|GetLight%20Indirect%20Intensity)))
    (:then_5
      (Class|SceneComponent|AddLocalTransform _sm_fridge_drawer (Math|Transform|MakeTransform (Math|Vector|MakeVector 0.0 (Variables|FRIDGEPARTS|GetDrawer%20Transform) 0.0) "0, 0, 0" "1,1,1") false false)
      (Transformation|SetMobility _sm_fridge_drawer (Variables|FRIDGEPARTS|GetDrawer%20Mobility)))))