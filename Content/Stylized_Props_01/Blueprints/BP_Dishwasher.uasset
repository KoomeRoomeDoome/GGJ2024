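; BP_Dishwasher is a dishwasher prop whose door and two baskets can be posed through variables.
; The construction script rolls the door by DoorAngle and slides the upper and bottom baskets along local Y by their own offsets.
; It also applies a shared Mobility setting to those three meshes.
; The event graph holds only disabled placeholder events, so the prop has no runtime logic.
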(event EventBeginPlay)

(event Collision|EventActorBeginOverlap
  (params (OtherActor :type Actor%20Object%20Reference)))

(event EventTick
  (params (DeltaSeconds :type Float%20%28single-precision%29)))

(fn ConstructionScript
  (bind _sm_dish_washer_basket (Variables|Default|GetSM_Dish_Washer_Basket))
  (Utilities|FlowControl|Sequence
    (:then_0
      (Transformation|AddLocalRotation (Variables|Default|GetSM_Dish_Washer_Door) (Math|Rotator|MakeRotator (Variables|DISHWASHERPARTS|GetDoor%20Angle) 0.0 0.0) false false))
    (:then_1
      (Class|SceneComponent|AddLocalTransform _sm_dish_washer_basket (Math|Transform|MakeTransform (Math|Vector|MakeVector 0.0 (Variables|DISHWASHERPARTS|GetUpper%20Basket%20Transform) 0.0) "0, 0, 0" "1,1,1") false false))
    (:then_2
      (Class|SceneComponent|AddLocalTransform (Variables|Default|GetSM_Dish_Washer_Basket1) (Math|Transform|MakeTransform (Math|Vector|MakeVector 0.0 (Variables|DISHWASHERPARTS|GetBottom%20Basket%20Transform) 0.0) "0, 0, 0" "1,1,1") false false)))
  (Transformation|SetMobility _sm_dish_washer_basket (Variables|DISHWASHERPARTS|GetMobility)))