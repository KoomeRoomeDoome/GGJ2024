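; Fluorescent light fixture prop pairing a mesh with a spot light, configurable per instance.
; The construction script applies exposed variables to mesh shadow casting, emissive brightness and color, and spot light shape, intensity, color, mobility and source size.
; When LightFlicker is enabled, Tick independently randomizes emissive brightness and light intensity each frame between zero and their set values.
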(event EventTick
  (params (DeltaSeconds :type Float%20%28single-precision%29))
  (if (Variables|FLUORESCENTPARAMETERS|GetLight%20Flicker)
    (Rendering|Material|SetScalarParameterValueonMaterials (Variables|Default|GetSM_Fluorescent_01) "Emissive_Brightness" (Math|Random|RandomFloatinRange 0.0 (Variables|FLUORESCENTPARAMETERS|GetEmissive%20Brightness)))
    (Rendering|Components|Light|SetIntensity (Variables|Default|GetSpotLight) (Math|Random|RandomFloatinRange 0.0 (Variables|FLUORESCENTPARAMETERS|GetLight%20Intensity)))))

(fn ConstructionScript
  (bind _spotlight (Variables|Default|GetSpotLight))
  (bind _sm_fluorescent_01 (Variables|Default|GetSM_Fluorescent_01))
  (Utilities|FlowControl|Sequence
    (:then_0
      (Rendering|SetCastShadow _sm_fluorescent_01 (Variables|FLUORESCENTPARAMETERS|GetFluorescent%20Mesh%20Shadow))
      (Rendering|Material|SetScalarParameterValueonMaterials _sm_fluorescent_01 "Emissive_Brightness" (Variables|FLUORESCENTPARAMETERS|GetEmissive%20Brightness))
      (Rendering|Material|SetVectorParameterValueonMaterials _sm_fluorescent_01 "Emissive Color Blend" (Math|Conversions|ToVector(LinearColor) (Math|Conversions|ToLinearColor(Color) (Variables|FLUORESCENTPARAMETERS|GetEmissive%20Color%20Blend)))))
    (:then_1
      (Rendering|Lighting|SetAttenuationRadius _spotlight (Variables|FLUORESCENTPARAMETERS|GetLight%20Radius))
      (Rendering|Lighting|SetOuterConeAngle _spotlight (Variables|FLUORESCENTPARAMETERS|GetLight%20Outer%20Cone))
      (Rendering|Lighting|SetInnerConeAngle _spotlight (Variables|FLUORESCENTPARAMETERS|GetLight%20Inner%20Cone))
      (Rendering|Components|Light|SetIntensity _spotlight (Variables|FLUORESCENTPARAMETERS|GetLight%20Intensity))
      (Rendering|Components|Light|SetLightColor _spotlight (Variables|FLUORESCENTPARAMETERS|GetLight%20Color) true)
      (Transformation|SetMobility _spotlight (Variables|FLUORESCENTPARAMETERS|GetLight%20Mobility))
      (Class|PointLightComponent|SetSoftSourceRadius _spotlight (Variables|FLUORESCENTPARAMETERS|GetSoft%20Source%20Radius))
      (Class|PointLightComponent|SetSourceRadius _spotlight (Variables|FLUORESCENTPARAMETERS|GetSource%20Radius))
      (Class|PointLightComponent|SetSourceLength _spotlight (Variables|FLUORESCENTPARAMETERS|GetSource%20Length))
      (Class|LightComponent|SetIndirectLightingIntensity _spotlight (Variables|FLUORESCENTPARAMETERS|GetLight%20Indirect%20Intensity)))))