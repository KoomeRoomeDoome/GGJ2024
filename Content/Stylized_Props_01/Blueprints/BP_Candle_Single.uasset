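; BP_Candle_Single is a configurable candle prop with a flame mesh and a point light.
; The construction script applies exposed variables to scale the flame mesh, set its material, and configure the light's brightness, color, radii, shadows, volumetric scattering and mobility.
; An optional light function material is assigned to the light when UseLightFunctions is enabled.
; The event graph is empty, so the blueprint adds no runtime logic.
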(event EventBeginPlay)

(event Collision|EventActorBeginOverlap
  (params (OtherActor :type Actor%20Object%20Reference)))

(event EventTick
  (params (DeltaSeconds :type Float%20%28single-precision%29)))

(fn ConstructionScript
  (bind _pointlight (Variables|Default|GetPointLight))
  (Utilities|FlowControl|Sequence
    (:then_0
      (Transformation|SetWorldScale3D (Variables|Default|GetSM_Candle_Flame) (Math|Vector|MakeVector (Variables|Default|GetFlame%20X%20Scale) (Variables|Default|GetFlame%20Y%20Scale) (Variables|Default|GetFlame%20Z%20Scale))))
    (:then_1
      (if (Variables|Default|GetUse%20Light%20Functions)
        (Rendering|Components|Light|SetLightFunctionMaterial _pointlight (Variables|Default|GetLight%20Function))))
    (:then_2
      (Rendering|Components|Light|SetIntensity _pointlight (Variables|Default|GetCandle%20Light%20Intensity))
      (Class|LightComponent|SetVolumetricScatteringIntensity _pointlight (Variables|Default|GetCandle%20Volumetric%20Light%20Intensity))
      (Rendering|Components|Light|SetCastShadows _pointlight (Variables|Default|GetCast%20Shadows))
      (Variables|/Script/Engine.LightComponent|SetContactShadowLength _pointlight (Variables|Default|GetContact%20Shadow%20Lenght))
      (Rendering|Lighting|SetAttenuationRadius _pointlight (Variables|Default|GetSet%20Attenuation%20Radius))
      (Class|LightComponentBase|SetCastVolumetricShadow _pointlight (Variables|Default|GetEnable%20Volumetric%20Shadows))
      (Rendering|Components|Light|SetLightColor _pointlight (Variables|Default|GetCandle%20Light%20Color) (Variables|Default|GetSRGB))
      (Class|LightComponent|SetIndirectLightingIntensity _pointlight (Variables|Default|GetIndirect%20Lighting%20Intensity))
      (Class|PointLightComponent|SetSourceRadius _pointlight (Variables|Default|GetSource%20Radius))
      (Class|PointLightComponent|SetSoftSourceRadius _pointlight (Variables|Default|GetSoft%20Soure%20Radius))
      (Transformation|SetMobility _pointlight (Variables|Default|GetCandle%20Light%20Mobility)))
    (:then_3
      (Rendering|Material|SetMaterial (Variables|Default|GetSM_Candle_Flame) 0 (Variables|Default|GetCandle%20Material)))))