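; Desk lamp prop with a static mesh and spot light, configurable per instance through exposed-looking variables.
; The construction script applies shadow casting and emissive brightness and color to the mesh materials, then pushes shape, intensity, color, mobility and source settings to the spot light.
; When LightFlicker is on, Tick randomizes emissive brightness and light intensity independently every frame, between zero and their configured maximums.
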(event EventTick
  (params (DeltaSeconds :type Float%20%28single-precision%29))
  (if (Variables|DESKLAMPPARAMETERS|GetLight%20Flicker)
    (Rendering|Material|SetScalarParameterValueonMaterials (Variables|Default|GetSM_Desk_Lamp) "Emissive_Brightness" (Math|Random|RandomFloatinRange 0.0 (Variables|DESKLAMPPARAMETERS|GetEmissive%20Brightness)))
    (Rendering|Components|Light|SetIntensity (Variables|Default|GetSpotLight) (Math|Random|RandomFloatinRange 0.0 (Variables|DESKLAMPPARAMETERS|GetLight%20Intensity)))))

(fn ConstructionScript
  (bind _spotlight (Variables|Default|GetSpotLight))
  (bind _sm_desk_lamp (Variables|Default|GetSM_Desk_Lamp))
  (Utilities|FlowControl|Sequence
    (:then_0
      (Rendering|SetCastShadow _sm_desk_lamp (Variables|DESKLAMPPARAMETERS|GetDesk%20Lamp%20Mesh%20Shadow))
      (Rendering|Material|SetScalarParameterValueonMaterials _sm_desk_lamp "Emissive_Brightness" (Variables|DESKLAMPPARAMETERS|GetEmissive%20Brightness))
      (Rendering|Material|SetVectorParameterValueonMaterials _sm_desk_lamp "Emissive Color Blend" (Math|Conversions|ToVector(LinearColor) (Math|Conversions|ToLinearColor(Color) (Variables|DESKLAMPPARAMETERS|GetEmissive%20Color%20Blend)))))
    (:then_1
      (Rendering|Lighting|SetAttenuationRadius _spotlight (Variables|DESKLAMPPARAMETERS|GetLight%20Radius))
      (Rendering|Lighting|SetOuterConeAngle _spotlight (Variables|DESKLAMPPARAMETERS|GetLight%20Outer%20Cone))
      (Rendering|Lighting|SetInnerConeAngle _spotlight (Variables|DESKLAMPPARAMETERS|GetLight%20Inner%20Cone))
      (Rendering|Components|Light|SetIntensity _spotlight (Variables|DESKLAMPPARAMETERS|GetLight%20Intensity))
      (Rendering|Components|Light|SetLightColor _spotlight (Variables|DESKLAMPPARAMETERS|GetLight%20Color) true)
      (Transformation|SetMobility _spotlight (Variables|DESKLAMPPARAMETERS|GetLight%20Mobility))
      (Class|PointLightComponent|SetSoftSourceRadius _spotlight (Variables|DESKLAMPPARAMETERS|GetSoft%20Source%20Radius))
      (Class|PointLightComponent|SetSourceRadius _spotlight (Variables|DESKLAMPPARAMETERS|GetSource%20Radius))
      (Class|PointLightComponent|SetSourceLength _spotlight (Variables|DESKLAMPPARAMETERS|GetSource%20Length))
      (Class|LightComponent|SetIndirectLightingIntensity _spotlight (Variables|DESKLAMPPARAMETERS|GetLight%20Indirect%20Intensity)))))