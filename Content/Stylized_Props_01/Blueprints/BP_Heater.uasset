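; BP_Heater is a configurable stylized heater prop with a mesh and a spot light for its glow.
; The construction script applies exposed variables to mesh shadow casting, emissive material parameters and the spot light's shape, color, intensity and mobility.
; When LightFlicker is on, Tick picks independent random emissive brightness and light intensity values between zero and their set maximums each frame, producing an unsmoothed flicker.
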(event EventTick
  (params (DeltaSeconds :type Float%20%28single-precision%29))
  (if (Variables|HEATERPARAMETERS|GetLight%20Flicker)
    (Rendering|Material|SetScalarParameterValueonMaterials (Variables|Default|GetSM_Heater) "Emissive_Brightness" (Math|Random|RandomFloatinRange 0.0 (Variables|HEATERPARAMETERS|GetEmissive%20Brightness)))
    (Rendering|Components|Light|SetIntensity (Variables|Default|GetSpotLight) (Math|Random|RandomFloatinRange 0.0 (Variables|HEATERPARAMETERS|GetLight%20Intensity)))))

(fn ConstructionScript
  (bind _sm_heater (Variables|Default|GetSM_Heater))
  (bind _spotlight (Variables|Default|GetSpotLight))
  (Utilities|FlowControl|Sequence
    (:then_0
      (Rendering|SetCastShadow _sm_heater (Variables|HEATERPARAMETERS|GetHeater%20Mesh%20Shadow))
      (Rendering|Material|SetScalarParameterValueonMaterials _sm_heater "Emissive_Brightness" (Variables|HEATERPARAMETERS|GetEmissive%20Brightness))
      (Rendering|Material|SetVectorParameterValueonMaterials _sm_heater "Emissive Color Blend" (Math|Conversions|ToVector(LinearColor) (Math|Conversions|ToLinearColor(Color) (Variables|HEATERPARAMETERS|GetEmissive%20Color%20Blend)))))
    (:then_1
      (Rendering|Lighting|SetAttenuationRadius _spotlight (Variables|HEATERPARAMETERS|GetResistance%20Glow%20Radius))
      (Rendering|Lighting|SetOuterConeAngle _spotlight (Variables|HEATERPARAMETERS|GetLight%20Outer%20Cone))
      (Rendering|Lighting|SetInnerConeAngle _spotlight (Variables|HEATERPARAMETERS|GetLight%20Inner%20Cone))
      (Rendering|Components|Light|SetIntensity _spotlight (Variables|HEATERPARAMETERS|GetLight%20Intensity))
      (Rendering|Components|Light|SetLightColor _spotlight (Variables|HEATERPARAMETERS|GetLight%20Color) true)
      (Transformation|SetMobility _spotlight (Variables|HEATERPARAMETERS|GetLight%20Mobility))
      (Class|PointLightComponent|SetSoftSourceRadius _spotlight (Variables|HEATERPARAMETERS|GetSoft%20Source%20Radius))
      (Class|PointLightComponent|SetSourceRadius _spotlight (Variables|HEATERPARAMETERS|GetSource%20Radius))
      (Class|PointLightComponent|SetSourceLength _spotlight (Variables|HEATERPARAMETERS|GetSource%20Length))
      (Class|LightComponent|SetIndirectLightingIntensity _spotlight (Variables|HEATERPARAMETERS|GetLight%20Indirect%20Intensity)))))