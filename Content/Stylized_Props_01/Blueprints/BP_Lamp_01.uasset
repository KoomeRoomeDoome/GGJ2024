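; BP_Lamp_01 is a configurable stylized lamp prop that pairs a lamp mesh with a spot light and can optionally flicker.
; The construction script applies exposed variables to the mesh's shadow casting and emissive material parameters, and to the spot light's shape, color, intensity, mobility, source size and contact shadows.
; When LightFlicker is enabled, Tick randomizes emissive brightness and light intensity every frame, each independently between zero and its configured value.
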(event EventTick
  (params (DeltaSeconds :type Float%20%28single-precision%29))
  (if (Variables|GROUNDLAMPPARAMETERS|GetLight%20Flicker)
    (Rendering|Material|SetScalarParameterValueonMaterials (Variables|Default|GetSM_Lamp_01) "Emissive_Brightness" (Math|Random|RandomFloatinRange 0.0 (Variables|GROUNDLAMPPARAMETERS|GetEmissive%20Brightness)))
    (Rendering|Components|Light|SetIntensity (Variables|Default|GetSpotLight) (Math|Random|RandomFloatinRange 0.0 (Variables|GROUNDLAMPPARAMETERS|GetLight%20Intensity)))))

(fn ConstructionScript
  (bind _spotlight (Variables|Default|GetSpotLight))
  (bind _sm_lamp_01 (Variables|Default|GetSM_Lamp_01))
  (Utilities|FlowControl|Sequence
    (:then_0
      (Rendering|SetCastShadow _sm_lamp_01 (Variables|GROUNDLAMPPARAMETERS|GetLamp%20Mesh%20Shadow))
      (Rendering|Material|SetScalarParameterValueonMaterials _sm_lamp_01 "Emissive_Brightness" (Variables|GROUNDLAMPPARAMETERS|GetEmissive%20Brightness))
      (Rendering|Material|SetVectorParameterValueonMaterials _sm_lamp_01 "Emissive Color Blend" (Math|Conversions|ToVector(LinearColor) (Math|Conversions|ToLinearColor(Color) (Variables|GROUNDLAMPPARAMETERS|GetEmissive%20Color%20Blend)))))
    (:then_1
      (Rendering|Lighting|SetAttenuationRadius _spotlight (Variables|GROUNDLAMPPARAMETERS|GetLight%20Radius))
      (Rendering|Lighting|SetOuterConeAngle _spotlight (Variables|GROUNDLAMPPARAMETERS|GetLight%20Outer%20Cone))
      (Rendering|Lighting|SetInnerConeAngle _spotlight (Variables|GROUNDLAMPPARAMETERS|GetLight%20Inner%20Cone))
      (Rendering|Components|Light|SetIntensity _spotlight (Variables|GROUNDLAMPPARAMETERS|GetLight%20Intensity))
      (Rendering|Components|Light|SetLightColor _spotlight (Variables|GROUNDLAMPPARAMETERS|GetLight%20Color) true)
      (Transformation|SetMobility _spotlight (Variables|GROUNDLAMPPARAMETERS|GetLight%20Mobility))
      (Class|PointLightComponent|SetSoftSourceRadius _spotlight (Variables|GROUNDLAMPPARAMETERS|GetSoft%20Source%20Radius))
      (Class|PointLightComponent|SetSourceRadius _spotlight (Variables|GROUNDLAMPPARAMETERS|GetSource%20Radius))
      (Class|PointLightComponent|SetSourceLength _spotlight (Variables|GROUNDLAMPPARAMETERS|GetSource%20Length))
      (Class|LightComponent|SetIndirectLightingIntensity _spotlight (Variables|GROUNDLAMPPARAMETERS|GetLight%20Indirect%20Intensity))
      (Variables|/Script/Engine.LightComponent|SetContactShadowLengthInWS _spotlight (Variables|GROUNDLAMPPARAMETERS|GetSet%20Contact%20Shadows%20in%20World%20Units))
      (Variables|/Script/Engine.LightComponent|SetContactShadowLength _spotlight (Variables|GROUNDLAMPPARAMETERS|GetContact%20Shadow%20Lenght)))))