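; Small cabinet prop with three drawer meshes that can be posed open or closed independently.
; The construction script offsets the top, middle and bottom drawers along local Y by their own variables, then applies a shared Mobility setting to all three after each offset.
; It has no runtime logic, as the event graph holds only disabled placeholder events.
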(event EventBeginPlay)

(event Collision|EventActorBeginOverlap
  (params (OtherActor :type Actor%20Object%20Reference)))

(event EventTick
  (params (DeltaSeconds :type Float%20%28single-precision%29)))

(fn ConstructionScript
  (bind _sm_small_cabinet_drawer1 (Variables|Default|GetSM_Small_Cabinet_Drawer1))
  (Utilities|FlowControl|Sequence
    (:then_0
      (Class|SceneComponent|AddLocalTransform (Variables|Default|GetSM_Small_Cabinet_Drawer) (Math|Transform|MakeTransform (Math|Vector|MakeVector 0.0 (Variables|Default|GetTop%20Drawer) 0.0) "0, 0, 0" "1,1,1") false false))
    (:then_1
      (Class|SceneComponent|AddLocalTransform _sm_small_cabinet_drawer1 (Math|Transform|MakeTransform (Math|Vector|MakeVector 0.0 (Variables|Default|GetMid%20Drawer) 0.0) "0, 0, 0" "1,1,1") false false))
    (:then_2
      (Class|SceneComponent|AddLocalTransform (Variables|Default|GetSM_Small_Cabinet_Drawer2) (Math|Transform|MakeTransform (Math|Vector|MakeVector 0.0 (Variables|Default|GetBottom%20Drawer) 0.0) "0, 0, 0" "1,1,1") false false)))
  (Transformation|SetMobility _sm_small_cabinet_drawer1 (Variables|Default|GetMobility)))