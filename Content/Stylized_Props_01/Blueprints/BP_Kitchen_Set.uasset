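; BP_Kitchen_Set is a stylized kitchen prop whose dishwasher door and baskets, cupboard doors and drawers are posed through per-part variables.
; The Construction Script offsets each part locally: doors rotate, with right-hand ones negated, while baskets and drawers slide along Y.
; Each step then applies a shared Mobility setting to all the movable meshes, including the drawer arranger.
; The event graph holds only disabled stubs, so the prop has no runtime behavior.
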(event EventBeginPlay)

(event Collision|EventActorBeginOverlap
  (params (OtherActor :type Actor%20Object%20Reference)))

(event EventTick
  (params (DeltaSeconds :type Float%20%28single-precision%29)))

(fn ConstructionScript
  (bind _sm_dish_washer_door (Variables|Default|GetSM_Dish_Washer_Door))
  (Utilities|FlowControl|Sequence
    (:then_0
      (Transformation|AddLocalRotation _sm_dish_washer_door (Math|Rotator|MakeRotator (Variables|Default|GetWasher%20Door%20Angle) 0.0 0.0) false false))
    (:then_1
      (Class|SceneComponent|AddLocalTransform (Variables|Default|GetSM_Dish_Washer_Basket) (Math|Transform|MakeTransform (Math|Vector|MakeVector 0.0 (Variables|Default|GetWasher%20Upper%20Basket) 0.0) "0, 0, 0" "1,1,1") false false))
    (:then_2
      (Class|SceneComponent|AddLocalTransform (Variables|Default|GetSM_Dish_Washer_Basket1) (Math|Transform|MakeTransform (Math|Vector|MakeVector 0.0 (Variables|Default|GetWasher%20Bottom%20Basket) 0.0) "0, 0, 0" "1,1,1") false false))
    (:then_3
      (Class|SceneComponent|AddLocalTransform (Variables|Default|GetSM_Cupboard_Top_Cap_L) (Math|Transform|MakeTransform "0, 0, 0" (Math|Rotator|MakeRotator 0.0 0.0 (Variables|Default|GetTop%20Cap%20Left)) "1,1,1") false false))
    (:then_4
      (Class|SceneComponent|AddLocalTransform (Variables|Default|GetSM_Cupboard_Top_Cap_R) (Math|Transform|MakeTransform "0, 0, 0" (Math|Rotator|MakeRotator 0.0 0.0 (* (Variables|Default|GetTop%20Cap%20Right) -1.0)) "1,1,1") false false))
    (:then_5
      (Class|SceneComponent|AddLocalTransform (Variables|Default|GetSM_Cupboard_Top_Cap_R1) (Math|Transform|MakeTransform "0, 0, 0" (Math|Rotator|MakeRotator 0.0 0.0 (* (Variables|Default|GetTop%20Cap%20Single) -1.0)) "1,1,1") false false))
    (:then_6
      (Class|SceneComponent|AddLocalTransform (Variables|Default|GetSM_Cupboard_Bot_Cap_L) (Math|Transform|MakeTransform "0, 0, 0" (Math|Rotator|MakeRotator 0.0 0.0 (Variables|Default|GetBottom%20Cap%20Left)) "1,1,1") false false))
    (:then_7
      (Class|SceneComponent|AddLocalTransform (Variables|Default|GetSM_Cupboard_Bot_Cap_R) (Math|Transform|MakeTransform "0, 0, 0" (Math|Rotator|MakeRotator 0.0 0.0 (* (Variables|Default|GetBottom%20Cap%20Right) -1.0)) "1,1,1") false false))
    (:then_8
      (Class|SceneComponent|AddLocalTransform (Variables|Default|GetSM_Cupboard_Drawer) (Math|Transform|MakeTransform (Math|Vector|MakeVector 0.0 (Variables|Default|GetDrawer%201) 0.0) "0, 0, 0" "1,1,1") false false))
    (:then_9
      (Class|SceneComponent|AddLocalTransform (Variables|Default|GetSM_Cupboard_Drawer1) (Math|Transform|MakeTransform (Math|Vector|MakeVector 0.0 (Variables|Default|GetDrawer%202) 0.0) "0, 0, 0" "1,1,1") false false))
    (:then_10
      (Class|SceneComponent|AddLocalTransform (Variables|Default|GetSM_Cupboard_Drawer2) (Math|Transform|MakeTransform (Math|Vector|MakeVector 0.0 (Variables|Default|GetDrawer%203) 0.0) "0, 0, 0" "1,1,1") false false))
    (:then_11
      (Class|SceneComponent|AddLocalTransform (Variables|Default|GetSM_Cupboard_Drawer3) (Math|Transform|MakeTransform (Math|Vector|MakeVector 0.0 (Variables|Default|GetDrawer%204) 0.0) "0, 0, 0" "1,1,1") false false)))
  (Transformation|SetMobility _sm_dish_washer_door (Variables|Default|GetMobility)))