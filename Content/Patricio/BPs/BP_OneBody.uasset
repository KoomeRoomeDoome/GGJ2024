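; BP_OneBody is a character body Blueprint that randomizes its appearance.
; The construction script picks torso and pants materials for slots 0 and 4 of one mesh, reveals a hat or one of two hairs, and tints Hair2 via a dynamic material.
; CustomizeCharacter repeats this on passed-in upper body, lower body and headwear components, tinting both hairs.
; The construction script's tint for Hair is disconnected.
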(fn ConstructionScript
  (bind _mesh (Variables|Character|GetMesh))
  ;[0.366 0.4658 1] Change Material Torso
  (Rendering|Material|SetMaterial _mesh 0 (.OutItem (Utilities|Array|Random (Variables|Default|GetTorsoMaterials))))
  (Rendering|SetVisibility (Utilities|Select :Index (Math|Random|RandomIntegerinRange 0 2) :Option%200 (Variables|Default|GetHat) :Option%201 (Variables|Default|GetHair2) :Option%202 (Variables|Default|GetHair)) true false)
  ;[0.02757 1 0.3387] Random Pants Material
  (Rendering|Material|SetMaterial _mesh 4 (.OutItem (Utilities|Array|Random (Variables|Default|GetPantsMaterials))))
  ;[1 0.4931 0.04779] Random Hair
  (bind _returnvalue (Rendering|Material|CreateDynamicMaterialInstance (Variables|Default|GetHair2) 0 0 "None" :!class /Script/Engine.PrimitiveComponent))
  (Rendering|Material|SetVectorParameterValue _returnvalue "HairColor" (Math|Color|MakeColor (Math|Random|RandomFloat) (Math|Random|RandomFloat) (Math|Random|RandomFloat)) :!class /Script/Engine.MaterialInstanceDynamic))

(fn CustomizeCharacter
  (params (Lower%20Body :type Skeletal%20Mesh%20Component%20Object%20Reference) (Upper%20Body :type Skeletal%20Mesh%20Component%20Object%20Reference) (Hair :type Static%20Mesh%20Component%20Object%20Reference) (Hair2 :type Static%20Mesh%20Component%20Object%20Reference) (Hat :type Static%20Mesh%20Component%20Object%20Reference))
  (Utilities|FlowControl|Sequence
    (:then_0
      ;[0.366 0.4658 1] Change Material Torso
      (Rendering|Material|SetMaterial Upper%20Body 0 (.OutItem (Utilities|Array|Random (Variables|Default|GetTorsoMaterials)))))
    (:then_1
      (Rendering|SetVisibility (Utilities|Select :Index (Math|Random|RandomIntegerinRange 0 2) :Option%200 Hair :Option%201 Hair2 :Option%202 Hat) true false))
    (:then_2
      ;[0.02757 1 0.3387] Random Pants Material
      (Rendering|Material|SetMaterial Lower%20Body 0 (.OutItem (Utilities|Array|Random (Variables|Default|GetPantsMaterials)))))
    (:then_3
      ;[1 0.4931 0.04779] Random Hair
      (bind _returnvalue (Rendering|Material|CreateDynamicMaterialInstance Hair2 0 0 "None" :!class /Script/Engine.PrimitiveComponent))
      (Rendering|Material|SetVectorParameterValue _returnvalue "HairColor" (Math|Color|MakeColor (Math|Random|RandomFloat) (Math|Random|RandomFloat) (Math|Random|RandomFloat)) :!class /Script/Engine.MaterialInstanceDynamic))
    (:then_4
      ;[1 0.4931 0.04779] Random Hair
      (bind _returnvalue_2 (Rendering|Material|CreateDynamicMaterialInstance Hair 0 0 "None" :!class /Script/Engine.PrimitiveComponent))
      (Rendering|Material|SetVectorParameterValue _returnvalue_2 "HairColor" (Math|Color|MakeColor (Math|Random|RandomFloat) (Math|Random|RandomFloat) (Math|Random|RandomFloat)) :!class /Script/Engine.MaterialInstanceDynamic))))