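; BP_DebugArray is a debug actor that lays out static meshes in configurable 3D grids.
; Its construction script loops over the values of the AssetList map, adding a hierarchical instanced static mesh component with each entry's mesh and transform.
; Each component receives a grid of instances sized by Count and spaced by the mesh's bounding box plus Offset.
; The event graph is unused.
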(event EventBeginPlay)

(event Collision|EventActorBeginOverlap
  (params (OtherActor :type Actor%20Object%20Reference)))

(event EventTick
  (params (DeltaSeconds :type Float%20%28single-precision%29)))

(fn ConstructionScript
  (bind _values (Utilities|Map|Values (Variables|Default|GetAssetList)))
  (for _array_element _values
    (bind _output_get (Variables|Default|SetCurrentData _array_element))
    (bind _returnvalue (AddComponent|AddHierarchicalInstancedStaticMeshComponent false (.transform _output_get)))
    (bind _output_get_2 (Variables|Default|SetCurrent%20HISM _returnvalue))
    (Components|StaticMesh|SetStaticMesh _output_get_2 (.mesh (Variables|Default|GetCurrentData)))
    ;[1 1 1] Count
    (for _index (range 0 (- (.X (Utilities|Struct|BreakIntVector (.count (Variables|Default|GetCurrentData)))) 1))
      (for _index_2 (range 0 (- (.Y (Utilities|Struct|BreakIntVector (.count (Variables|Default|GetCurrentData)))) 1))
        (for _index_3 (range 0 (- (.Z (Utilities|Struct|BreakIntVector (.count (Variables|Default|GetCurrentData)))) 1))
          (Components|InstancedStaticMesh|AddInstance (Variables|Default|GetCurrent%20HISM) (Math|Transform|MakeTransform (Math|Vector|MakeVector (* _index (+ (.x (- (.max (StaticMesh|GetBoundingBox (.mesh (Variables|Default|GetCurrentData)))) (.min (StaticMesh|GetBoundingBox (.mesh (Variables|Default|GetCurrentData)))))) (.X (Math|Vector|BreakVector (.offset (Variables|Default|GetCurrentData)))))) (* _index_2 (+ (.y (- (.max (StaticMesh|GetBoundingBox (.mesh (Variables|Default|GetCurrentData)))) (.min (StaticMesh|GetBoundingBox (.mesh (Variables|Default|GetCurrentData)))))) (.Y (Math|Vector|BreakVector (.offset (Variables|Default|GetCurrentData)))))) (* _index_3 (+ (.z (- (.max (StaticMesh|GetBoundingBox (.mesh (Variables|Default|GetCurrentData)))) (.min (StaticMesh|GetBoundingBox (.mesh (Variables|Default|GetCurrentData)))))) (.Z (Math|Vector|BreakVector (.offset (Variables|Default|GetCurrentData)))))))) false))))))