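; Restroom trigger actor that signals a game pause while the player is inside it and a resume when they leave.
; Overlaps on PauseBounds filtered by the Player tag set PlayerInPause and fire OnPause or OnResume on both itself and GS_GameState.
; Entering also tells the referenced enemy spawner to clean bodies from the map and spawn enemies.
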(event OnComponentBeginOverlap(PauseBounds)
  (params (OverlappedComponent :type Primitive%20Component%20Object%20Reference) (OtherActor :type Actor%20Object%20Reference) (OtherComp :type Primitive%20Component%20Object%20Reference) (OtherBodyIndex :type Integer) (bFromSweep :type Boolean) (SweepResult :type Hit%20Result%20Structure%20%28by%20ref%29))
  (bind _enemyspawnerreference (Variables|Default|GetEnemySpawnerReference))
  (if (Actor|ActorHasTag OtherActor "Player")
    (Variables|Default|SetPlayerInPause true)
    (Default|CallOnPause)
    (bind _asgs_game_state (Utilities|Casting|CastToGS_GameState (Game|GetGameState)))
    (Default|CallOnPause _asgs_game_state)
    (Default|CleanMapfromBodies _enemyspawnerreference)
    (Default|SpawnEnemies _enemyspawnerreference)))

(event OnComponentEndOverlap(PauseBounds)
  (params (OverlappedComponent :type Primitive%20Component%20Object%20Reference) (OtherActor :type Actor%20Object%20Reference) (OtherComp :type Primitive%20Component%20Object%20Reference) (OtherBodyIndex :type Integer))
  (if (Actor|ActorHasTag OtherActor "Player")
    (Variables|Default|SetPlayerInPause false)
    (Default|CallOnResume)
    (bind _asgs_game_state (Utilities|Casting|CastToGS_GameState (Game|GetGameState)))
    (Default|CallOnResume _asgs_game_state)))

(fn ConstructionScript)