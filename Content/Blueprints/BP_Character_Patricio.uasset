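; Patricio character Blueprint with a modular body (lower body, hands, upper body) following the main mesh's pose, driven by physical animation.
; On BeginPlay it simulates bodies below a configured bone and enters mixed ragdoll, blending physics with animation using separate leg weights.
; A full ragdoll function disables capsule collision, simulates the whole mesh and lowers physical animation strength.
; SetArmsWeight is never called here, and AddDrink is an empty stub.
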(event EventBeginPlay
  (CallFunction|SetupPhysicalAnimation))

(fn ConstructionScript
  (Components|SkinnedMesh|SetLeaderPoseComponent (Variables|Default|GetLowerBody) (Variables|Character|GetMesh) false false))

(fn SetupPhysicalAnimation
  (Class|PhysicalAnimationComponent|SetSkeletalMeshComponent (Variables|Default|GetPhysicalAnimation) (Variables|Character|GetMesh))
  (Class|PhysicalAnimationComponent|ApplyPhysicalAnimationSettingsBelow (Variables|Default|GetPhysicalAnimation) (Variables|PhysicalAnimation|GetPhysicalAnimationBodyName) (Variables|PhysicalAnimation|GetPhysical%20Animation%20Data) false)
  (Class|SkeletalMeshComponent|SetAllBodiesBelowSimulatePhysics (Variables|Character|GetMesh) (Variables|PhysicalAnimation|GetPhysicalAnimationBodyName) true false)
  (CallFunction|DoMixedRagdoll))

(fn SetArmsWeight
  ;[1 1 1] Setting different weights to the legs
  (Class|SkeletalMeshComponent|SetAllBodiesBelowPhysicsBlendWeight (Variables|Character|GetMesh) (Utilities|Name|MakeLiteralName "clavicle_l") (Variables|PhysicalAnimation|GetLegs%20Physics%20Blend%20Weight) false true)
  (Class|SkeletalMeshComponent|SetAllBodiesBelowPhysicsBlendWeight (Variables|Character|GetMesh) (Utilities|Name|MakeLiteralName "clavicle_r") (Variables|PhysicalAnimation|GetLegs%20Physics%20Blend%20Weight) false true))

(fn AddDrink)

(fn DoFullRagdoll
  (Collision|SetCollisionEnabled (Variables|Collision|GetCapsuleComponent) "NoCollision")
  (Physics|SetSimulatePhysics (Variables|Character|GetMesh) true)
  (Class|SkeletalMeshComponent|SetAllBodiesBelowSimulatePhysics (Variables|Character|GetMesh) (Variables|PhysicalAnimation|GetPhysicalAnimationBodyName) true true)
  (Variables|Behaviour|SetIsRagdolling true)
  (Class|PhysicalAnimationComponent|SetStrengthMultiplyer (Variables|Default|GetPhysicalAnimation) 1.0))

(fn DoMixedRagdoll
  (Variables|Behaviour|SetIsRagdolling false)
  (Collision|SetCollisionEnabled (Variables|Collision|GetCapsuleComponent) "QueryOnly")
  (Physics|SetSimulatePhysics (Variables|Character|GetMesh) false)
  (Class|SkeletalMeshComponent|SetAllBodiesBelowSimulatePhysics (Variables|Character|GetMesh) (Variables|PhysicalAnimation|GetPhysicalAnimationBodyName) true false)
  (Class|SkeletalMeshComponent|SetAllBodiesPhysicsBlendWeight (Variables|Character|GetMesh) (Variables|PhysicalAnimation|GetMaster%20Physics%20Blend%20Weight) false)
  ;[1 1 1] Setting different weights to the legs
  (Class|SkeletalMeshComponent|SetAllBodiesBelowPhysicsBlendWeight (Variables|Character|GetMesh) (Utilities|Name|MakeLiteralName "thigh_l") (Variables|PhysicalAnimation|GetLegs%20Physics%20Blend%20Weight) false true)
  (Class|SkeletalMeshComponent|SetAllBodiesBelowPhysicsBlendWeight (Variables|Character|GetMesh) (Utilities|Name|MakeLiteralName "thigh_r") (Variables|PhysicalAnimation|GetLegs%20Physics%20Blend%20Weight) false true)
  (Class|PhysicalAnimationComponent|SetStrengthMultiplyer (Variables|Default|GetPhysicalAnimation) 5.0))