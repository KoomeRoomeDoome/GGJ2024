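; Base character Blueprint providing physics-driven animation, a montage attack and overridable hooks for child classes such as enemies.
; On BeginPlay, Physical Animation starts a mixed ragdoll that simulates bodies below a configured bone, with separate blend weights for legs.
; Full ragdoll lowers physical animation strength and disables capsule collision; returning to mixed saves a pose snapshot and restores both.
; Attacks are locked until the montage completes, and ThrowSetup enables gravity and probe collision.
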(event Custom|Attack
  (if (not (Variables|Behaviour|GetIsAttacking))
    (Variables|Behaviour|SetIsAttacking true)
    (Animation|Montage|PlayMontage (Variables|Character|GetMesh) "/Game/Blueprints/Characters/Montages/AM_Attack3.AM_Attack3" 1.5
      (:OnCompleted
        (Variables|Behaviour|SetIsAttacking false)
        (CallFunction|DoneAttacking)))))

(event Custom|DoneAttacking
  ;[1 1 1] override with specific behaviour
)

(event Custom|WasThrown
  ;[1 1 1] override in enemy to restore
)

(event EventBeginPlay
  (CallFunction|SetupPhysicalAnimation))

(fn ConstructionScript)

(fn SetupPhysicalAnimation
  (Class|PhysicalAnimationComponent|SetSkeletalMeshComponent (Variables|Default|GetPhysicalAnimation) (Variables|Character|GetMesh))
  (Class|PhysicalAnimationComponent|ApplyPhysicalAnimationSettingsBelow (Variables|Default|GetPhysicalAnimation) (Variables|PhysicalAnimation|GetPhysicalAnimationBodyName) (Variables|PhysicalAnimation|GetPhysical%20Animation%20Data) false)
  (Class|SkeletalMeshComponent|SetAllBodiesBelowSimulatePhysics (Variables|Character|GetMesh) (Variables|PhysicalAnimation|GetPhysicalAnimationBodyName) true false)
  (Variables|Default|SetMeshRelativePosition (Transformation|GetRelativeTransform (Variables|Character|GetMesh)))
  (CallFunction|DoMixedRagdoll))

(fn SetArmsWeight
  ;[1 1 1] Setting different weights to the legs
  (Class|SkeletalMeshComponent|SetAllBodiesBelowPhysicsBlendWeight (Variables|Character|GetMesh) (Utilities|Name|MakeLiteralName "clavicle_l") (Variables|PhysicalAnimation|GetLegs%20Physics%20Blend%20Weight) false true)
  (Class|SkeletalMeshComponent|SetAllBodiesBelowPhysicsBlendWeight (Variables|Character|GetMesh) (Utilities|Name|MakeLiteralName "clavicle_r") (Variables|PhysicalAnimation|GetLegs%20Physics%20Blend%20Weight) false true))

(fn AddDrink)

(fn DoFullRagdoll
  (if (not (Variables|Behaviour|GetIsRagdolling))
    (Variables|Behaviour|SetIsRagdolling true)
    (Class|PhysicalAnimationComponent|SetStrengthMultiplyer (Variables|Default|GetPhysicalAnimation) 1.0)
    (Collision|SetCollisionEnabled (Variables|Collision|GetCapsuleComponent) "NoCollision")))

(fn DoMixedRagdoll
  (Class|AnimInstance|SavePoseSnapshot (Components|SkeletalMesh|GetAnimInstance (Variables|Character|GetMesh)) "RagdollFinalPose")
  (Variables|Behaviour|SetIsRagdolling false)
  (Class|SkeletalMeshComponent|SetAllBodiesBelowSimulatePhysics (Variables|Character|GetMesh) (Variables|PhysicalAnimation|GetPhysicalAnimationBodyName) true false)
  (Class|SkeletalMeshComponent|SetAllBodiesPhysicsBlendWeight (Variables|Character|GetMesh) (Variables|PhysicalAnimation|GetMaster%20Physics%20Blend%20Weight) false)
  ;[1 1 1] Setting different weights to the legs
  (Class|SkeletalMeshComponent|SetAllBodiesBelowPhysicsBlendWeight (Variables|Character|GetMesh) (Utilities|Name|MakeLiteralName "thigh_l") (Variables|PhysicalAnimation|GetLegs%20Physics%20Blend%20Weight) false true)
  (Class|SkeletalMeshComponent|SetAllBodiesBelowPhysicsBlendWeight (Variables|Character|GetMesh) (Utilities|Name|MakeLiteralName "thigh_r") (Variables|PhysicalAnimation|GetLegs%20Physics%20Blend%20Weight) false true)
  (Class|PhysicalAnimationComponent|SetStrengthMultiplyer (Variables|Default|GetPhysicalAnimation) 5.0)
  (Collision|SetCollisionEnabled (Variables|Collision|GetCapsuleComponent) "QueryOnly"))

(fn DoAttack
  (CallFunction|Attack))

(fn ThrowSetup
  (Physics|SetEnableGravity (Variables|Collision|GetCapsuleComponent) true)
  (Collision|SetCollisionEnabled (Variables|Collision|GetCapsuleComponent) "QueryAndProbe"))