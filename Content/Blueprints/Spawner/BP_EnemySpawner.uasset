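; Wave spawner that fills each wave with three batches of ranked enemies from per-wave data, placed at sequential, then random locations.
; A looping timer lets a random living enemy attack while the game state is in Aggro.
; Deaths advance the batch when survivors hit a threshold accumulated from 33% of each batch size.
; With none left and Aggro off, it shows the restroom widget and ends the wave; tracked corpses can be cleared.
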(event Custom|SpawnEnemies
  ;[1 0 0] Call to start waves
  (bind (_batch_info _batch) (CallFunction|GetBatchSpawnNumber))
  (CallFunction|SpawnBatch _batch_info _batch)
  (CallFunction|UpdateRemainingEnemiestoStartBatchat _batch_info))

(event Custom|EnemyDead
  (bind _spawnedenemies (Variables|Default|GetSpawnedEnemies))
  (bind _returnvalue (Utilities|Array|Length _spawnedenemies))
  (if (== _returnvalue (Variables|Default|GetRemainingEnemiesToStartBatchAt))
    (switch Utilities|FlowControl|Switch|SwitchonE_Batch (Variables|/Game/Blueprints/GS_GameState.GS_GameState_C|GetBatch (Variables|Default|GetGameState))
      (:NewEnumerator0
        _)
      (:NewEnumerator1
        _))
    ;[1 1 1] notify the game state that the batch has changed (and others who might be interested)
    (Default|NextBatch (Variables|Default|GetGameState))
    ;[1 1 1] Proceed spawning new batch
    (CallFunction|SpawnEnemies)
    (elif (and (== _returnvalue 0) (not (Variables|/Game/Blueprints/GS_GameState.GS_GameState_C|GetAggro (Variables|Default|GetGameState))))
      (bind _returnvalue_2 (UserInterface|CreateWidget "/Game/DrunkBar/UI/W_GoToRestroom.W_GoToRestroom_C" (Game|GetPlayerController 0)))
      (UserInterface|Viewport|AddtoViewport _returnvalue_2 0)
      (Default|TriggerEndWave (Variables|Default|GetGameState)))))

(event Custom|AttackSelectionTick
  (bind _spawnedenemies (Variables|Default|GetSpawnedEnemies))
  (bind _outitem (Utilities|Array|Random _spawnedenemies))
  ;[1 1 1] Sets a random attacker from the active ones
  (if (Variables|/Game/Blueprints/GS_GameState.GS_GameState_C|GetAggro (Variables|Default|GetGameState))
    (Utilities|IsValid _outitem
      (:Is%20Valid
        (Default|SetCanAttack _outitem)))))

(event EventBeginPlay
  (bind _asgs_game_state (Utilities|Casting|CastToGS_GameState (Game|GetGameState)))
  (Variables|Default|SetGameState _asgs_game_state)
  (CallFunction|SpawnEnemies)
  ;[1 1 1] Sets a random attacker from the active ones
  (Utilities|Time|SetTimerbyEvent (delegate Custom|AttackSelectionTick) (Variables|Default|GetAttackSelectionFrequency) true))

(fn ConstructionScript)

(fn SpawnBatch
  (params (Batch%20Info :type S%20Batch%20Spawn%20Structure) (Batch :type E_Batch%20Enum :default "NewEnumerator0"))
  (bind (_weak _medium _strong _boss) (Utilities|Struct|BreakS_BatchSpawn Batch%20Info))
  (CallFunction|SpawnEnemyNumber _weak "NewEnumerator0" Batch)
  (CallFunction|SpawnEnemyNumber _medium "NewEnumerator1" Batch)
  (CallFunction|SpawnEnemyNumber _strong "NewEnumerator2" Batch)
  (CallFunction|SpawnEnemyNumber _boss "NewEnumerator3" Batch))

(fn GetBatchSpawnNumber
  (bind _wavesspawndata (Variables|Default|GetWavesSpawnData))
  (bind _gamestate (Variables|Default|GetGameState))
  (bind _gamestate_2 (Variables|Default|GetGameState))
  (bind _currentwave (Variables|/Game/Blueprints/GS_GameState.GS_GameState_C|GetCurrentWave _gamestate_2))
  (bind _batch (Variables|/Game/Blueprints/GS_GameState.GS_GameState_C|GetBatch _gamestate))
  (bind _returnvalue (Math|Conversions|ToInteger(Byte) _currentwave))
  (bind _output (Utilities|Array|Get(acopy) _wavesspawndata _returnvalue))
  (switch Utilities|FlowControl|Switch|SwitchonE_Batch _batch
    (:NewEnumerator0
      (return (Variables|/Game/Blueprints/Spawner/PDA_WaveSpawn.PDA_WaveSpawn_C|GetBatch1 _output) _batch))
    (:NewEnumerator1
      (return (Variables|/Game/Blueprints/Spawner/PDA_WaveSpawn.PDA_WaveSpawn_C|GetBatch2 _output) _batch))
    (:NewEnumerator2
      (return (Variables|/Game/Blueprints/Spawner/PDA_WaveSpawn.PDA_WaveSpawn_C|GetBatch3 _output) _batch))))

(fn SpawnEnemyNumber
  (params (Number :type Integer) (Rank :type E_EnemyRank%20Enum :default "NewEnumerator0") (Batch :type E_Batch%20Enum :default "NewEnumerator0"))
  (if (> Number 0)
    (for _index (range 1 Number)
      (bind _transform (CallFunction|GetSpawnLocation Batch))
      (bind _enemy (Utilities|SpawnSpecificEnemy _transform Rank)
        (:Out
          (EventDispatchers|BindEventtoOnDeath _enemy (EventDispatchers|CreateEvent :!event CalledonEnemyDeath))
          (Utilities|Array|AddUnique (Variables|Default|GetSpawnedEnemies) _enemy))))))

(fn UpdateRemainingEnemiestoStartBatchat
  (params (New%20batch :type S%20Batch%20Spawn%20Structure))
  (Variables|Default|SetRemainingEnemiesToStartBatchAt (+ (Math|Float|Truncate (* (+ (.weak New%20batch) (.medium New%20batch) (.strong New%20batch) (.boss New%20batch)) 0.33)) (Variables|Default|GetRemainingEnemiesToStartBatchAt))))

(fn GetSpawnLocation
  (params (Batch :type E_Batch%20Enum :default "NewEnumerator0"))
  (switch Utilities|FlowControl|Switch|SwitchonE_Batch Batch
    (:NewEnumerator0
      (LocalVariables|SetBatchLocation (Utilities|Array|Get(acopy) (Variables|Default|GetFirstbatchesLocations) (Variables|Default|GetFirstbatchLocationIndex)))
      (Math|Integer|IncrementInt (Variables|Default|GetFirstbatchLocationIndex)
        (:%20%20
          _)))
    (:NewEnumerator1
      (LocalVariables|SetBatchLocation (Utilities|Array|Get(acopy) (Variables|SpawnConfiguration|GetNewBatchesLocations) (Math|Random|RandomIntegerinRange 0 (- (Utilities|Array|Length (Variables|SpawnConfiguration|GetNewBatchesLocations)) 1))) :!label _label))
    (:NewEnumerator2
      (goto _label)))
  (bind _output_get (LocalVariables|SetBatchLocation (Math|Transform|MakeTransform (+ (Transformation|GetActorLocation) (.location (LocalVariables|GetBatchLocation))) (.rotation (LocalVariables|GetBatchLocation)) (.scale (LocalVariables|GetBatchLocation)))))
  (return _output_get))

(fn CalledonEnemyDeath
  (params (DeadEnemy :type BP%20Character%20Object%20Reference))
  (bind _spawnedenemies (Variables|Default|GetSpawnedEnemies))
  (bind _asbp_character_enemy_base (Utilities|Casting|CastToBP_Character_Enemy_Base DeadEnemy))
  (Utilities|Array|AddUnique (Variables|Default|GetDeadEnemies) (Utilities|Array|Get(acopy) (Variables|Default|GetSpawnedEnemies) (Utilities|Array|FindItem _spawnedenemies _asbp_character_enemy_base)))
  (Utilities|Array|RemoveItem _spawnedenemies _asbp_character_enemy_base)
  (CallFunction|EnemyDead))

(fn CleanMapfromBodies
  (for _array_element (Variables|Default|GetDeadEnemies)
    (Utilities|IsValid _array_element
      (:Is%20Valid
        (Actor|DestroyActor _array_element)))))