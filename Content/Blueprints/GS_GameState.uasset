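; Game state that tracks wave-based aggression: the current wave and batch, whether aggro is active, and pause status.
; TriggerAggro starts a wave once, resetting the batch and adding a new W_UI widget to the viewport.
; TriggerEndWave clears aggro and advances the wave enum, while NextBatch steps through batches within a wave, both stopping at a final value.
; Event dispatchers broadcast wave start and end, batch changes, pause and resume to listeners.
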(event Custom|TriggerAggro
  ;[1 0.3229 0.3229] Call this method to start the wave of aggression, the spiral of violence, the madness...
  (if (not (Variables|Default|GetAggro))
    (Variables|Default|SetBatch "NewEnumerator0")
    (Default|CallOnWaveStart (Variables|Default|GetCurrentWave))
    (Variables|Default|SetAggro true)
    (bind _returnvalue (UserInterface|CreateWidget "/Game/DrunkBar/UI/W_UI.W_UI_C" (Game|GetPlayerController 0)))
    (UserInterface|Viewport|AddtoViewport _returnvalue 0)))

(event Custom|TriggerEndWave
  ;[0.1587 0.3906 0.1261] Call this when the wave is  over
  (Variables|Default|SetAggro false)
  (Default|CallOnWaveEnd)
  (CallFunction|IncreaseWave))

(event Custom|NextBatch
  ;[1 1 1] Update batch
  (Development|PrintString (Utilities|String|Append (Utilities|String|MakeLiteralString "Current Batch: ") (Utilities|String|EnumtoString (Variables|Default|GetBatch))))
  (Development|PrintString (Utilities|String|Append (Utilities|String|MakeLiteralString "Current Batch: ") (Utilities|String|EnumtoString (Variables|Default|GetCurrentWave))))
  (switch Utilities|FlowControl|Switch|SwitchonE_Batch (Variables|Default|GetBatch)
    (:NewEnumerator0
      _)
    (:NewEnumerator1
      _))
  (Variables|Default|SetBatch (Utilities|Enum|ByteToEnumE_Batch (+ (Variables|Default|GetBatch) 1)))
  (Default|CallOnNextBatch))

(event Custom|GamePaused
  (Default|CallOnPause)
  (Variables|Default|SetPause true))

(event Custom|GameResumed
  (Default|CallOnResume)
  (Variables|Default|SetPause false))

(fn ConstructionScript)

(fn IncreaseWave
  (switch Utilities|FlowControl|Switch|SwitchonE_Wave (Variables|Default|GetCurrentWave)
    (:NewEnumerator0
      _)
    (:NewEnumerator1
      _)
    (:NewEnumerator2
      _)
    (:NewEnumerator3
      _))
  (Variables|Default|SetCurrentWave (Utilities|Enum|ByteToEnumE_Wave (+ (Variables|Default|GetCurrentWave) 1)))
  (Variables|Default|SetBatch "NewEnumerator0"))