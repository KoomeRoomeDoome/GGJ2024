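; Base enemy character that targets the player, can carry a stealable drink, and aggros when the GameState starts a wave.
; Mirrors aggro, target and attack permission into its AI controller's blackboard to drive behavior.
; Damage type separates punch kills from delayed throw deaths, with surviving thrown enemies restored to mixed ragdoll after a delay.
; Death launches a physics ragdoll along player forward; full ragdoll also triggers GameState aggro.
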(event OnComponentBeginOverlap(CapsuleComponent)
  (params (OverlappedComponent :type Primitive%20Component%20Object%20Reference) (OtherActor :type Actor%20Object%20Reference) (OtherComp :type Primitive%20Component%20Object%20Reference) (OtherBodyIndex :type Integer) (bFromSweep :type Boolean) (SweepResult :type Hit%20Result%20Structure%20%28by%20ref%29))
  (if (Actor|ActorHasTag OtherActor "Player")
    _))

(event Custom|ActivateWave
  ;[1 1 1] Call when the combat system is ready
  (bind _asgs_game_state (Utilities|Casting|CastToGS_GameState (Game|GetGameState)))
  (Default|TriggerAggro _asgs_game_state))

(event Custom|GetPissedOff
  (params (Wave :type E_Wave%20Enum :default "NewEnumerator0"))
  (Variables|Behaviour|SetAggroed true)
  (bind _asaic_enemy_base (Utilities|Casting|CastToAIC_EnemyBase (Pawn|GetController)))
  (AI|Components|Blackboard|SetValueasBool (AI|GetBlackboard _asaic_enemy_base) (Utilities|Name|MakeLiteralName "Aggroed") true))

(event Custom|SetCanAttack
  ;[1 1 1] Manage AI attack allowance
  (Variables|Default|SetCanAttack true)
  (bind _asaic_enemy_base (Utilities|Casting|CastToAIC_EnemyBase (Pawn|GetController)))
  (AI|Components|Blackboard|SetValueasBool (AI|GetBlackboard _asaic_enemy_base) (Utilities|Name|MakeLiteralName "CanAttack") true))

(event Custom|SetTarget
  (bind _asaic_enemy_base (Utilities|Casting|CastToAIC_EnemyBase (Pawn|GetController)))
  (AI|Components|Blackboard|SetValueasObject (AI|GetBlackboard _asaic_enemy_base) (Utilities|Name|MakeLiteralName "TargetActor") (Game|Player|GetPlayerPawn 0)))

(event EventBeginPlay
  (|CallParentFunction)
  (Variables|health|SetHealth (Variables|health|GetMaxHealth))
  (bind _asgs_game_state (Utilities|Casting|CastToGS_GameState (Game|GetGameState)))
  (EventDispatchers|BindEventtoOnWaveStart _asgs_game_state (delegate Custom|GetPissedOff))
  (bind _output_get (Variables|Behaviour|SetAggroed (Variables|/Game/Blueprints/GS_GameState.GS_GameState_C|GetAggro _asgs_game_state)))
  (if _output_get
    (CallFunction|GetPissedOff (Variables|/Game/Blueprints/GS_GameState.GS_GameState_C|GetCurrentWave _asgs_game_state)))
  (CallFunction|SetTarget)
  (if (not (Variables|Default|GetHasDrink))
    (Components|DestroyComponent (Variables|Default|GetStaticMesh))))

(event EventDoneAttacking
  ;[1 1 1] Manage AI attack allowance
  (Variables|Default|SetCanAttack false)
  (bind _asaic_enemy_base (Utilities|Casting|CastToAIC_EnemyBase (Pawn|GetController)))
  (AI|Components|Blackboard|SetValueasBool (AI|GetBlackboard _asaic_enemy_base) (Utilities|Name|MakeLiteralName "CanAttack") false))

(event Game|Damage|EventAnyDamage
  (params (Damage :type Float%20%28single-precision%29) (DamageType :type Damage%20Type%20Object%20Reference) (InstigatedBy :type Controller%20Object%20Reference) (DamageCauser :type Actor%20Object%20Reference))
  ;[1 0.1406 0.1406] Damage management
  (if (Variables|Default|GetCanBeHit)
    (bind _remaininghealth (Utilities|AddDamage Damage))
    (if (<= _remaininghealth 0.0)
      ;[1 1 1] Deaths! above is death from deadly punch, below is death from superspeed throw of justice(R)
      (Utilities|Casting|CastToDT_Punch DamageType
        (:then
          (CallFunction|Death))
        (:CastFailed
          (Variables|Default|SetIsDead true)
          (Utilities|FlowControl|Delay 1.0)
          (CallFunction|RestoreEnemy)
          (CallFunction|Death)))
      (else
        ;[1 1 1] This is damage without death, above is from throw and below from punch
        (Utilities|Casting|CastToDT_Thrown DamageType)
        (Utilities|FlowControl|Delay (Variables|Default|GetThrownRestoreTime))
        (CallFunction|RestoreEnemy)))))

(fn ConstructionScript
  (|CallParentFunction))

(fn DoFullRagdoll
  (|CallParentFunction)
  (CallFunction|ActivateWave)
  (Pawn|Components|CharacterMovement|DisableMovement (Variables|Character|GetCharacterMovement)))

(fn DoMixedRagdoll
  (|CallParentFunction)
  (Pawn|Components|CharacterMovement|SetMovementMode (Variables|Character|GetCharacterMovement) "MOVE_Walking" 0))

(fn DrinkStolen
  (if (Variables|Default|GetHasDrink)
    (Components|DestroyComponent (Variables|Default|GetStaticMesh))
    (Variables|Default|SetHasDrink false)))

(fn RestoreEnemy
  (bind _mesh (Variables|Character|GetMesh))
  (Physics|SetSimulatePhysics (Variables|Default|GetCapsuleComponent) false)
  (CallFunction|DoMixedRagdoll)
  (Transformation|AttachComponentToComponent _mesh (Variables|Transformation|GetRootComponent) "" "KeepRelative" "KeepRelative" "KeepRelative" true)
  (Transformation|SetRelativeTransform _mesh (Variables|Default|GetMeshRelativePosition) false true))

(fn Death
  (bind _mesh (Variables|Character|GetMesh))
  (bind _mesh_2 (Variables|Character|GetMesh))
  ;[1 1 1] 1...2...3... DING DING DING!!!
  (|CallParentFunction)
  (Class|Pawn|DetachfromControllerPendingDestroy)
  (CallFunction|DoFullRagdoll)
  (Class|SkeletalMeshComponent|SetAllBodiesSimulatePhysics _mesh true)
  (Physics|SetEnableGravity _mesh true)
  (Physics|SetSimulatePhysics _mesh_2 true)
  (Class|SkeletalMeshComponent|AddImpulsetoAllBodiesBelow _mesh_2 (* (Transformation|GetActorForwardVector (Game|Player|GetPlayerPawn 0)) 6e+02) "spine_01" true true)
  (Components|DestroyComponent (Variables|Default|GetCapsuleComponent)))