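; BP_Character_Enemy_Weak is a weak enemy character Blueprint that randomizes its appearance on construction.
; After running the parent construction script, it applies a random entry from PantsMaterials to one mesh material slot.
; It also creates a dynamic material instance on the Hair2 component and sets its HairColor parameter to a random RGB color.
; The event graph holds only disabled placeholder events, so it adds no runtime logic of its own.
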(event EventBeginPlay
  (|CallParentFunction) ; This node is disabled and will not be called.\nDrag off pins to build functionality.
)

(event Collision|EventActorBeginOverlap
  (params (OtherActor :type Actor%20Object%20Reference)))

(event EventTick
  (params (DeltaSeconds :type Float%20%28single-precision%29)))

(fn ConstructionScript
  (|CallParentFunction)
  ;[0.02757 1 0.3387] Random Pants Material
  (Rendering|Material|SetMaterial (Variables|Character|GetMesh) 4 (.OutItem (Utilities|Array|Random (Variables|Default|GetPantsMaterials))))
  ;[1 0.4931 0.04779] Random Hair
  (bind _returnvalue (Rendering|Material|CreateDynamicMaterialInstance (Variables|Default|GetHair2) 0 0 "None" :!class /Script/Engine.PrimitiveComponent))
  (Rendering|Material|SetVectorParameterValue _returnvalue "HairColor" (Math|Color|MakeColor (Math|Random|RandomFloat) (Math|Random|RandomFloat) (Math|Random|RandomFloat)) :!class /Script/Engine.MaterialInstanceDynamic))